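; BP_Projectile is a homing attack projectile that chases a single target and applies physical damage on contact.
; Each tick it offsets the root component toward the target's current location without sweeping, using the ProjectileMovement component's InitialSpeed.
; When its collision component begins overlapping that target, only the authority applies damage with the attacker as damage causer, then destroys the projectile.
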(event `self.ReceiveTick`
  (params (DeltaSeconds :type "Float (single-precision)"))
  (bind _targettoattack (`self.TargetToAttack`))
  (`/Engine/EditorBlueprintResources/StandardMacros.IsValid` _targettoattack
    (:`Is Valid`
      (`SceneComponent.K2_AddWorldOffset` (`self.DefaultSceneRoot`) (* DeltaSeconds (* (`KismetMathLibrary.Normal` (- (`self.K2_GetActorLocation` _targettoattack) (`self.K2_GetActorLocation`))) (`ProjectileMovementComponent.InitialSpeed` (`self.ProjectileMovement`)))) false false))))

(event `self.Collision.OnComponentBeginOverlap`
  (params (OverlappedComponent :type "PrimitiveComponent Object Reference") (OtherActor :type "Actor Object Reference") (OtherComp :type "PrimitiveComponent Object Reference") (OtherBodyIndex :type Integer) (bFromSweep :type Boolean) (SweepResult :type "HitResult Structure (by ref)"))
  (if (and (== OtherActor (`self.TargetToAttack`)) (`self.HasAuthority`))
    (`GameplayStatics.ApplyDamage` (`self.TargetToAttack`) (`self.ProjectileDamage`) null (`self.Attacker`) "/Game/LOL/Character/ActorComponents/HealthSystem/Blueprint/BP_ApplyDamageType_Physical.BP_ApplyDamageType_Physical_C")
    (`self.K2_DestroyActor`)))

(fn `UserConstructionScript`)