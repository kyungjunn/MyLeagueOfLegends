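; BP_Projectile_Q is a projectile actor in the character attack system, apparently for a Q ability, that flies straight along its forward vector.
; Each tick it copies Speed into ProjectileMovement.InitialSpeed, then manually offsets the root by that speed times delta time, without sweep.
; Tick also resets the lifespan to two seconds every frame, so that timer never expires while ticking.
; The graph holds no hit or damage logic.
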(event `self.ReceiveTick`
  (params (DeltaSeconds :type "Float (single-precision)"))
  (bind _output_get (set `ProjectileMovementComponent.InitialSpeed` (`self.Speed`) (`self.ProjectileMovement`)))
  (`SceneComponent.K2_AddWorldOffset` (`self.DefaultSceneRoot`) (* DeltaSeconds (* (`self.GetActorForwardVector`) _output_get)) false false)
  (`self.SetLifeSpan` 2.0))

(fn `UserConstructionScript`
  (`parent.UserConstructionScript`))