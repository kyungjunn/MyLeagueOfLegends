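; Attacker component for LOL characters that carries out a melee or ranged attack on the current target.
; AttackTarget checks that TargetToAttack is valid, then branches on AttackType.
; Melee applies physical damage immediately, while Ranged spawns the supplied projectile class and passes it the target, damage and movement speed.
; Ranged damage is left to the projectile, and the event graph has no active logic.
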(fn `AttackTarget`
  (params (Projectile :type "Transform Structure"))
  (bind _projectilespeed (`self.ProjectileSpeed`))
  (`/Engine/EditorBlueprintResources/StandardMacros.IsValid` (`self.TargetToAttack`)
    (:`Is Valid`
      (switch `/Game/LOL/Character/ActorComponents/AttackSystem/Enum/E_AttackType` (`self.AttackType`)
        (:`NewEnumerator0`
          ; 근접이면 바로 Apply Damage
          (`GameplayStatics.ApplyDamage` (`self.TargetToAttack`) (`self.AttackDamage`) null null "/Game/LOL/Character/ActorComponents/HealthSystem/Blueprint/BP_ApplyDamageType_Physical.BP_ApplyDamageType_Physical_C"))
        (:`NewEnumerator1`
          ; 원거리면 물체 날려서 물체에서 Apply Damage
          (bind _returnvalue (`|SpawnActorFromClass` (`self.Projectile`) Projectile "Undefined" "MultiplyWithRoot" null null))
          (bind _asbp_projectile (cast `/Game/LOL/Character/ActorComponents/AttackSystem/Projectile/BP_Projectile` _returnvalue))
          (set `/Game/LOL/Character/ActorComponents/AttackSystem/Projectile/BP_Projectile.TargetToAttack` (`self.TargetToAttack`) _asbp_projectile)
          (set `/Game/LOL/Character/ActorComponents/AttackSystem/Projectile/BP_Projectile.ProjectileDamage` (`self.AttackDamage`) _asbp_projectile)
          (bind _projectilemovement (`/Game/LOL/Character/ActorComponents/AttackSystem/Projectile/BP_Projectile.ProjectileMovement` _asbp_projectile))
          (set `ProjectileMovementComponent.InitialSpeed` _projectilespeed _projectilemovement)
          (set `ProjectileMovementComponent.MaxSpeed` _projectilespeed _projectilemovement))))))