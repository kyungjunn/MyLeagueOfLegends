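; Health component that tracks replicated HP for its owning actor and broadcasts HP updates through a RepNotify.
; C2S damage events reduce damage by physical or magic resistance, leaving true damage untouched, then lower HP.
; Lethal damage calls an empty death event, fires OnDeath and destroys the owner.
; RegenerateHP restores HP up to the maximum, but its looping timer setup is unconnected, so regeneration never starts.
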(event `self.ReceiveBeginPlay`
  (set `self.CurrentHP` (`self.MaxHP`)))

(event `C2S_Player_Death`)

(event `C2S_TakeDamage`
  (params (DamageAmount :type "Float (double-precision)") (DamageType :type "DamageType Object Reference"))
  (bind _returndamage (`self.ApplyResistance` DamageAmount DamageType))
  (bind _returnvalue (- (`self.CurrentHP`) _returndamage))
  (if (<= _returnvalue 0.0)
    (`self.C2S_Player_Death`)
    (`self.OnDeath`)
    (`Actor.K2_DestroyActor` (`self.GetOwner`))
    (else
      (set `self.CurrentHP` _returnvalue)
      (`KismetSystemLibrary.K2_UnPauseTimerHandle` (`self.RegenerationTimerHandler`)))))

(fn `ApplyResistance`
  (params (DamageAmount :type "Float (double-precision)") (DamageType :type "DamageType Object Reference"))
  (returns (ReturnDamage :type "Float (double-precision)"))
  (locals (CalculateDamage :type "Float (double-precision)"))
  (bind _asbp_apply_damage_type (cast `/Game/LOL/Character/ActorComponents/HealthSystem/Blueprint/BP_ApplyDamageType` DamageType))
  (bind _damagetype (`/Game/LOL/Character/ActorComponents/HealthSystem/Blueprint/BP_ApplyDamageType.GetDamageType` _asbp_apply_damage_type))
  (switch `/Game/LOL/Character/ActorComponents/HealthSystem/Enum/E_DamageType` _damagetype
    (:`NewEnumerator0`
      (set `local.CalculateDamage` DamageAmount))
    (:`NewEnumerator1`
      (set `local.CalculateDamage` (- DamageAmount (* (/ DamageAmount 100.0) (`self.PhysicsDamageResistance`)))))
    (:`NewEnumerator2`
      (set `local.CalculateDamage` (- DamageAmount (* (/ DamageAmount 100.0) (`self.MagicDamageResistance`))))))
  (return (`local.CalculateDamage`)))

(fn `OnRep_CurrentHP`
  (`self.OnHPUpdate` (`self.CurrentHP`)))

(fn `RegenerateHP`
  (bind _returnvalue (+ (`self.CurrentHP`) (`self.HPRegeneration`)))
  (if (>= _returnvalue (`self.MaxHP`))
    (set `self.CurrentHP` (`self.MaxHP`))
    (`KismetSystemLibrary.K2_PauseTimerHandle` (`self.RegenerationTimerHandler`))
    (`self.OnHealthRegenerated`)
    (else
      (set `self.CurrentHP` _returnvalue)
      (`self.OnHealthRegenerated`))))