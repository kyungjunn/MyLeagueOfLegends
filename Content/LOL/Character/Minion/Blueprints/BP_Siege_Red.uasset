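; Red-team siege minion Blueprint that plays its attack animation when the minion attacks.
; On BeginPlay it binds a handler to the OnMinionAttack event, after running the parent logic.
; The handler calls C2S_AttackAnim, which relays to S2M_AttackAnim to play the attack montage on the mesh, a chain named for client-to-server-to-multicast replication.
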(event `self.ReceiveBeginPlay`
  (`parent.ReceiveBeginPlay`)
  (add `self.OnMinionAttack` (delegate `MinionAttack`)))

(event `C2S_AttackAnim`
  (`self.S2M_AttackAnim`))

(event `MinionAttack`
  (`self.C2S_AttackAnim`))

(event `S2M_AttackAnim`
  (`|PlayMontage` (`self.Mesh`) "/Game/LOL/Character/Minion/Siegn/Team_Red/Animations/AM_Siege_Red_Attack.AM_Siege_Red_Attack" 1.0 0.0 "Default"))

(fn `UserConstructionScript`
  (`parent.UserConstructionScript`))