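; BP_Minion is the minion character for a LOL-style game, with a health component, an overhead health bar and a patrol point reference.
; On BeginPlay it stores the BP_MinionPatrolPoint found in the level and hands its health component to its WBP_PlayerHealthBar widget.
; AnyDamage prints the amount and forwards it to the health component's C2STakeDamage.
; OnArrivedToPatrolPoint is an empty stub, with an unconnected AIC_Minion cast.
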(event `self.ReceiveAnyDamage`
  (params (Damage :type "Float (single-precision)") (DamageType :type "DamageType Object Reference") (InstigatedBy :type "Controller Object Reference") (DamageCauser :type "Actor Object Reference"))
  (`KismetSystemLibrary.PrintString` (`KismetStringLibrary.Conv_DoubleToString` Damage))
  (`/Game/LOL/Character/ActorComponents/HealthSystem/BP_HealthComponent.C2S_TakeDamage` (`self.BP_HealthPointsComponent`) Damage DamageType))

(event `self.ReceiveBeginPlay`
  ; 초기화
  ;; 정찰 위치 액터 저장
  (bind _returnvalue (`GameplayStatics.GetActorOfClass` "/Game/LOL/Character/Minion/Blueprints/BP_MinionPatrolPoint.BP_MinionPatrolPoint_C"))
  (set `self.PatrolPoints` _returnvalue)
  ;; 미니언 개별 HealthComponent 전달
  (bind _aswbp_player_health_bar (cast `/Game/LOL/UI/Characters/WBP_PlayerHealthBar` (`WidgetComponent.GetUserWidgetObject` (`self.MinionHealthWidget`))))
  (`/Game/LOL/UI/Characters/WBP_PlayerHealthBar.Set` _aswbp_player_health_bar (`self.BP_HealthPointsComponent`)))

(fn `OnArrivedToPatrolPoint`
  (params (NewPatrolPoint :type "/Game/LOL/Character/Minion/Blueprints/BP_MinionPatrolPoint Object Reference")))

(fn `UserConstructionScript`)