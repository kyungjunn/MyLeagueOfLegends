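; BP_MinionSpawner spawns waves of BP_Minion actors at its own transform, apparently for a LOL-style game.
; The MInionSpawner event delays the first InitMinionWave, which starts a looping timer that calls SpawnMinion at short intervals.
; SpawnMinion counts spawns and, at MaxSpawnCount, pauses that timer, resets the count and schedules InitMinionWave on a looping timer for the next wave.
; Nothing in this graph calls MInionSpawner.
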(event `MInionSpawner`
  ; Minion Spawn
  ;; 미니언 웨이브 처음 생성 시간
  (`KismetSystemLibrary.K2_SetTimerDelegate` (delegate `InitMinionWave`) 10.0))

(event `InitMinionWave`
  ; Minion Spawn
  (bind _returnvalue (`KismetSystemLibrary.K2_SetTimerDelegate` (delegate `SpawnMinion`) 1.5 true))
  (set `self.SpawnTimerHandle` _returnvalue))

(event `SpawnMinion`
  ; Minion Spawn
  (`|SpawnActorFromClass` "/Game/LOL/Character/Minion/BP_Minion.BP_Minion_C" (`self.GetTransform`) "Undefined" "MultiplyWithRoot" null null)
  ;; 미니언 카운트 증가
  (set `self.SpawnCount` (+ (`self.SpawnCount`) 1))
  ;; 미니언 6마리 생성했는가
  (if (>= (`self.SpawnCount`) (`self.MaxSpawnCount`))
    (`KismetSystemLibrary.K2_PauseTimerHandle` (`self.SpawnTimerhandle`))
    ;; 미니언 카운트 0 초기화, 다시 웨이브 시작
    (set `self.SpawnCount` 0)
    (`KismetSystemLibrary.K2_SetTimerDelegate` (delegate `InitMinionWave`) 10.0 true)))

(fn `UserConstructionScript`)