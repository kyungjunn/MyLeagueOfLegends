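; BP_Minion is a minion character that takes damage, displays its health and holds a reference to a patrol point.
; On BeginPlay it stores a BP_MinionPatrolPoint found in the level and passes its own health component to its WBP_MinionHealth widget.
; Incoming damage is printed, then forwarded to BPHealthPointsComponent.
; OnArrivedToPatrolPoint is an empty stub, with an unconnected AIC_Minion cast left in the asset.
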(event `self.ReceiveAnyDamage`
  (params (Damage :type "Float (single-precision)") (DamageType :type "DamageType Object Reference") (InstigatedBy :type "Controller Object Reference") (DamageCauser :type "Actor Object Reference"))
  (`KismetSystemLibrary.PrintString` (`KismetStringLibrary.Conv_DoubleToString` Damage))
  (`/Game/LOL/Character/ActorComponents/HealthSystem/BP_HealthPointsComponent.TakeDamage` (`self.BP_HealthPointsComponent`) Damage DamageType))

(event `self.ReceiveBeginPlay`
  ; 초기화
  ;; 정찰 위치 액터 저장
  (bind _returnvalue (`GameplayStatics.GetActorOfClass` "/Game/LOL/Character/Minion/BP_MinionPatrolPoint.BP_MinionPatrolPoint_C"))
  (set `self.PatrolPoints` _returnvalue)
  ;; 미니언 개별 HealthComponent 전달
  (bind _aswbp_minion_health (cast `/Game/LOL/Character/UI/WBP_MinionHealth` (`WidgetComponent.GetUserWidgetObject` (`self.MinionHealthWidget`))))
  (set `/Game/LOL/Character/UI/WBP_MinionHealth.MinionHealthComponent` (`self.BP_HealthPointsComponent`) _aswbp_minion_health))

(fn `OnArrivedToPatrolPoint`
  (params (NewPatrolPoint :type "/Game/LOL/Character/Minion/BP_MinionPatrolPoint Object Reference")))

(fn `UserConstructionScript`)