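; Ezreal champion Blueprint for a LoL-style game, handling basic attacks, damage intake and gold income.
; BeginPlay sets up the health bar, a one-second gold timer and a paused attack timer.
; Tick stops movement and unpauses attacks when the target minion is within capsule-adjusted range.
; Attacks and damage go through attacker and health components, with montages relayed client-to-server-to-multicast; the minion death gold reward is unconnected.
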(event `BeginAttack`
  ; 매 초마다 나의 골드가 증가 / 공격
  (`/Game/LOL/Character/ActorComponents/AttackSystem/BP_AttackerComponent.C2S_AttackDamage` (`self.BP_AttackerComponent`) (`SceneComponent.K2_GetComponentToWorld` (`self.Projectile`)) self (`/Game/LOL/Character/ActorComponents/AttackSystem/BP_AttackerComponent.TargetToAttack` (`self.BP_AttackerComponent`)))
  (`self.CTS_AttackAnim`))

(event `CTS_AttackAnim`
  ; Client -> Server 에 알려주기
  (`self.STM_AttackAnim`))

(event `ResetAttackTimer`
  ; 매 초마다 나의 골드가 증가 / 공격
  (bind _returnvalue (`KismetSystemLibrary.K2_SetTimerDelegate` (delegate `BeginAttack`) (`/Game/LOL/Character/ActorComponents/AttackSystem/BP_AttackerComponent.AttackRate` (`self.BP_AttackerComponent`)) true false -1.0 :!label _label))
  (bind _output_get (set `self.AttackTimerHandle` _returnvalue))
  (`KismetSystemLibrary.K2_PauseTimerHandle` _output_get))

(event `self.ReceiveBeginPlay`
  ; 매 초마다 나의 골드가 증가 / 공격
  (bind _asbp_player_controller (cast `/Game/LOL/Core/Framework/BP_PlayerController` (`GameplayStatics.GetPlayerController` 0)))
  (set `self.PlayerControllerRef` _asbp_player_controller)
  (bind _aswbp_player_health_bar (cast `/Game/LOL/UI/Characters/WBP_PlayerHealthBar` (`WidgetComponent.GetUserWidgetObject` (`self.PlayerHealthBar`))))
  (`/Game/LOL/UI/Characters/WBP_PlayerHealthBar.Set` _aswbp_player_health_bar (`self.BP_HealthPointsComponent`))
  (bind _returnvalue (`GameplayStatics.GetActorOfClass` "/Game/LOL/Character/Minion/Blueprints/BP_Minion.BP_Minion_C"))
  (set `self.MinionRef` _returnvalue)
  (`KismetSystemLibrary.K2_SetTimerDelegate` (delegate `AutoIncreaseMoney`) 1.0 true)
  (goto _label))

(event `AutoIncreaseMoney`
  ; 매 초마다 나의 골드가 증가 / 공격
  (set `self.Money` (+ (`self.Money`) 1))
  (`self.ShowMeTheMoney`))

(event `STM_AttackAnim`
  ; Server -> Multicast  Attack Montage 뿌려주기
  (`|PlayMontage` (`self.Mesh`) "/Game/LOL/Character/Champions/Ezreal/Animations/AM_EzrealAttack.AM_EzrealAttack" 1.0 0.0 "Attack1"))

(event `KillMinion`)

(event `self.ReceiveAnyDamage`
  (params (Damage :type "Float (single-precision)") (DamageType :type "DamageType Object Reference") (InstigatedBy :type "Controller Object Reference") (DamageCauser :type "Actor Object Reference"))
  ; 공격을 받았을 때
  (`KismetSystemLibrary.PrintString` (`KismetStringLibrary.Conv_DoubleToString` Damage))
  (`/Game/LOL/Character/ActorComponents/HealthSystem/BP_HealthComponent.C2S_TakeDamage` (`self.BP_HealthPointsComponent`) Damage DamageType))

(event `self.ReceiveTick`
  (params (DeltaSeconds :type "Float (single-precision)"))
  (bind _targettoattack (`/Game/LOL/Character/ActorComponents/AttackSystem/BP_AttackerComponent.TargetToAttack` (`self.BP_AttackerComponent`)))
  ; 사거리 안에 공격
  (`/Engine/EditorBlueprintResources/StandardMacros.IsValid` _targettoattack
    (:`Is Valid`
      (bind _result (`self.TargetInRange` _targettoattack))
      (if _result
        (`MovementComponent.StopMovementImmediately` (`self.CharacterMovement`))
        (`KismetSystemLibrary.K2_UnPauseTimerHandle` (`self.AttackTimerHandle`))))))

(event `SetMoney`
  (set `self.Money` (+ (`/Game/LOL/Character/Minion/Blueprints/BP_Minion.MinionValue` (`self.MinionRef`)) (`self.Money`))))

(fn `SpendMoney`
  (params (Money :type Integer))
  (returns (`Remaining Money` :type Integer))
  (bind _output_get (set `self.Money` (- (`self.Money`) Money)))
  (return _output_get))

(fn `TargetInRange`
  (params (`Other Target` :type "Actor Object Reference"))
  (returns (Result :type Boolean))
  (bind _asbp_minion (cast `/Game/LOL/Character/Minion/Blueprints/BP_Minion` `Other Target`))
  (`/Engine/EditorBlueprintResources/StandardMacros.IsValid` `Other Target`
    (:`Is Valid`
      (return (<= (`self.GetDistanceTo` self `Other Target`) (+ (`CapsuleComponent.CapsuleRadius` (`Character.CapsuleComponent` _asbp_minion)) (`CapsuleComponent.CapsuleRadius` (`self.CapsuleComponent`)) (`/Game/LOL/Character/ActorComponents/AttackSystem/BP_AttackerComponent.AttackRange` (`self.BP_AttackerComponent`))))))))

(fn `UserConstructionScript`
  (`parent.UserConstructionScript`))