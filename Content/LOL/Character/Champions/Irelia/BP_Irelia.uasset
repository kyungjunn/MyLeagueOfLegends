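; Character Blueprint for the champion Irelia that runs a looping automatic attack.
; On BeginPlay, after the parent's, a repeating timer fires BeginAttack at the stat component's attack rate after an initial delay.
; Each attack sends the attacker component's current target to its damage call without checking it here, then requests the animation.
; The animation request passes through C2S and S2M events, named as client-to-server and server-to-multicast, to play Irelia's attack montage.
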(event `self.C2S_AttackAnim`
  (`self.S2M_AttackAnim`))

(event `self.BeginAttack`
  (`/Game/LOL/Character/ActorComponents/AttackSystem/BP_AttackerComponent.C2S_AttackDamage` :`self` (`self.BP_AttackerComponent`) :`Attaker` self :`TargetActor` (`/Game/LOL/Character/ActorComponents/AttackSystem/BP_AttackerComponent.TargetToAttack` (`self.BP_AttackerComponent`)))
  (`self.C2S_AttackAnim`))

(event `self.ReceiveBeginPlay`
  (`parent.ReceiveBeginPlay`)
  (`KismetSystemLibrary.K2_SetTimerDelegate` (delegate `self.BeginAttack`) (`StatComponent.AttackRate` (`self.BP_StatComponent`)) true false 1.0))

(event `self.S2M_AttackAnim`
  (`|PlayMontage` (`self.Mesh`) "/Game/LOL/Character/Champions/Irelia/Animations/AM_IreliaAttack.AM_IreliaAttack" 1.0 0.0 "Default"))

(fn `UserConstructionScript`
  (`parent.UserConstructionScript`))