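; BP_PlayerController is a player controller that manages the in-game store UI and initializes the player's inventory.
; On BeginPlay it creates the WBP_Store widget, resizes the BP_Player inventory component's slots to InventorySize, then adds the store to the viewport hidden.
; The IA_OpenShore input action toggles the store's visibility through the ShowStore and HideStore events.
; If the player character is not a BP_Player, setup stops before the store reaches the viewport.
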(event `self.ReceiveBeginPlay`
  ; 기본 HUD 생성
  (`parent.ReceiveBeginPlay`)
  (bind _returnvalue (`|CreateWidget` "/Game/LOL/Store/Widgets/WBP_Store.WBP_Store_C"))
  (set `self.WBP Store` _returnvalue)
  (bind _asbp_player (cast `/Game/LOL/Characters/BP_Player` (`GameplayStatics.GetPlayerCharacter` 0)))
  (`KismetArrayLibrary.Array_Resize` (`/Game/LOL/Store/Blueprints/BP_InventoryComponent.Slots` (`/Game/LOL/Characters/BP_Player.BP_InventoryComponent` _asbp_player)) (`self.InventorySize`))
  (`UserWidget.AddToViewport` (`self.WBP Store`) 0)
  (`self.HideStore`))

(event `HideStore`
  ; Hide Store
  (`Widget.SetVisibility` (`self.WBP Store`) "Hidden"))

(event `EnhancedInput|/Game/TopDown/Input/Actions/IA_OpenShore`
  (params (ActionValue :type Boolean) (ElapsedSeconds :type "Float (double-precision)") (TriggeredSeconds :type "Float (double-precision)") (InputAction :type "InputAction Object Reference" :default "/Game/TopDown/Input/Actions/IA_OpenShore.IA_OpenShore"))
  ; Store Button (P)
  (:`Triggered`
    (if (`|EnumEquality` (`Widget.GetVisibility` (`self.WBP Store`)) "Visible")
      (`self.HideStore`)
      (else
        (`self.ShowStore`)))))

(event `ShowStore`
  ; Show Store
  (`Widget.SetVisibility` (`self.WBP Store`) "Visible"))

(fn `UserConstructionScript`
  (`parent.UserConstructionScript`))