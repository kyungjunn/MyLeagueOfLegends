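; BP_Player is the player Blueprint that holds the Money balance and grants passive gold income over time.
; On BeginPlay it caches the store and inventory widgets from BP_PlayerController and starts a looping one-second timer.
; Each tick of that timer increments Money and refreshes the wallet display in both widgets.
; SpendMoney is meant to deduct an amount and return the balance, without refreshing either widget.
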(event `self.ReceiveBeginPlay`
  ; 매 초마다 나의 골드가 증가
  (bind _asbp_player_controller (cast `/Game/LOL/Characters/BP_PlayerController` (`GameplayStatics.GetPlayerController` 0)))
  (bind _wbp_store (`/Game/LOL/Characters/BP_PlayerController.WBP Store` _asbp_player_controller))
  (set `self.WBP Store` _wbp_store)
  (set `self.WBP Inventory` (`/Game/LOL/Store/Widgets/WBP_Store.WBP_Inventory` _wbp_store))
  (`KismetSystemLibrary.K2_SetTimerDelegate` (delegate `AutoIncreaseMoney`) 1.0 true))

(event `AutoIncreaseMoney`
  ; 매 초마다 나의 골드가 증가
  (set `self.Money` (+ (`self.Money`) 1))
  (`/Game/LOL/Store/Widgets/WBP_Store.UpdatePlayerWallet` (`self.WBP Store`))
  (`/Game/LOL/Store/Widgets/WBP_Inventory.UpdatePlayerWalletInInventory` (`self.WBP Inventory`)))

(fn `SpendMoney`
  (params (Money :type Integer))
  (returns (`Remaining Money` :type Integer))
  (bind _output_get (set `self.Money` (- (`self.Money`) Money)))
  (return _output_get))

(fn `UserConstructionScript`
  (`parent.UserConstructionScript`))