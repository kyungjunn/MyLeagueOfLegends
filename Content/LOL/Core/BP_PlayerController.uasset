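; Player controller for a League of Legends-style top-down game, handling click movement, cursor feedback and the player HUD.
; On BeginPlay the local controller creates the health and store widgets and sizes the pawn's inventory; an input toggles the store.
; Held clicks follow the cursor, while short clicks path to the point and can clear the attack target.
; Tick shows a crosshair cursor over minions; attack inputs are empty stubs.
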(event `self.ReceiveBeginPlay`
  ; 초기화
  (if (`self.IsLocalPlayerController`)
    (`parent.ReceiveBeginPlay`)
    (bind _returnvalue (`|CreateWidget` "/Game/LOL/UI/Characters/WBP_PlayerDetailHealth.WBP_PlayerDetailHealth_C" null (`/Game/LOL/Character/Champions/Ezreal/BP_Ezreal.BP_HealthPointsComponent` (`self.PlayerRef`))))
    (set `self.PlayerHealth` _returnvalue)
    (bind _returnvalue_2 (`|CreateWidget` "/Game/LOL/UI/Store/WBP_Store.WBP_Store_C"))
    (set `self.WBP Store` _returnvalue_2)
    (`KismetArrayLibrary.Array_Resize` (`/Game/LOL/Store/Blueprints/BP_InventoryComponent.Slots` (`/Game/LOL/Character/Champions/Ezreal/BP_Ezreal.BP_InventoryComponent` (`self.PlayerRef`))) (`self.InventorySize`))
    (`UserWidget.AddToViewport` (`self.PlayerHealth`) 0)
    (`UserWidget.AddToViewport` (`self.WBP Store`) 1)
    (`self.HideStore`)))

(event `EnhancedInput|/Game/TopDown/Input/Actions/IA_OpenShore`
  (params (ActionValue :type Boolean) (ElapsedSeconds :type "Float (double-precision)") (TriggeredSeconds :type "Float (double-precision)") (InputAction :type "InputAction Object Reference" :default "/Game/TopDown/Input/Actions/IA_OpenShore.IA_OpenShore"))
  ; Store Button (P)
  (:`Triggered`
    (if (`Widget.IsVisible` (`self.WBP Store`))
      (`self.HideStore`)
      (else
        (`self.ShowStore`)))))

(event `HideStore`
  ; Hide Store
  (`Widget.SetVisibility` (`self.WBP Store`) "Hidden"))

(event `ShowStore`
  ; Show Store
  (`Widget.SetVisibility` (`self.WBP Store`) "Visible"))

(event `self.ReceiveTick`
  (params (DeltaSeconds :type "Float (single-precision)"))
  ; 마우스 커서의 대상이 미니언이면 커서 변경
  (`self.UpdateMouseCursor`))

(event `EnhancedInput|/Game/TopDown/Input/Actions/IA_SetDestination_Click`
  (params (ActionValue :type Boolean) (ElapsedSeconds :type "Float (double-precision)") (TriggeredSeconds :type "Float (double-precision)") (InputAction :type "InputAction Object Reference" :default "/Game/TopDown/Input/Actions/IA_SetDestination_Click.IA_SetDestination_Click"))
  (bind (_hit _location) (`self.GetLocationUnderCursor`))
  (bind (_hit_2 _location_2) (`self.GetLocationUnderCursor`))
  (bind _playerref (`self.PlayerRef`))
  ; TopDown Move
  (:`Triggered`
    (if _hit
      (bind _output_get (set `self.CachedDestination` _location))
      (`self.Follow` _output_get)))
  (:`Started`
    (`self.StopMovement`)
    (if _hit_2
      (set `self.CachedDestination` _location_2)))
  (:`Canceled`
    (if (< ElapsedSeconds (`self.PressedThreshold`)) :!label _label
      (`self.MoveTo` (`self.CachedDestination`))
      (if (`self.bIsNotAttackClick`)
        (set `/Game/LOL/Character/ActorComponents/AttackSystem/BP_AttackerComponent.TargetToAttack` null (`/Game/LOL/Character/Champions/Ezreal/BP_Ezreal.BP_AttackerComponent` _playerref))
        (`/Game/LOL/Character/Champions/Ezreal/BP_Ezreal.ResetAttackTimer` _playerref))))
  (:`Completed`
    (goto _label)))

(event `EnhancedInput|/Game/TopDown/Input/Actions/IA_PreAttackKey`
  (params (ActionValue :type Boolean) (ElapsedSeconds :type "Float (double-precision)") (TriggeredSeconds :type "Float (double-precision)") (InputAction :type "InputAction Object Reference" :default "/Game/TopDown/Input/Actions/IA_PreAttackKey.IA_PreAttackKey")))

(event `EnhancedInput|/Game/TopDown/Input/Actions/IA_AttackClick`
  (params (ActionValue :type Boolean) (ElapsedSeconds :type "Float (double-precision)") (TriggeredSeconds :type "Float (double-precision)") (InputAction :type "InputAction Object Reference" :default "/Game/TopDown/Input/Actions/IA_AttackClick.IA_AttackClick")))

(fn `UpdateMouseCursor`
  (bind (_bblockinghit _binitialoverlap _time _distance _location _impactpoint _normal _impactnormal _physmat _hitactor) (`GameplayStatics.BreakHitResult` (`self.GetHitResultUnderCursorByChannel` "TraceTypeQuery1")))
  (if _bblockinghit
    (cast `/Game/LOL/Character/Minion/Blueprints/BP_Minion` _hitactor
      (:`then`
        ; 공격 커서
        (set `self.CurrentMouseCursor` "Crosshairs"))
      (:`CastFailed`
        ; 일반 커서
        (set `self.CurrentMouseCursor` "Default")))))

(fn `UserConstructionScript`
  (`parent.UserConstructionScript`))