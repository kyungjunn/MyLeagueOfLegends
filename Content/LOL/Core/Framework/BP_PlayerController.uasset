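; Player controller for a LoL-style top-down game, handling UI, movement, attack and skill input.
; Local BeginPlay shows champion select; Client_OnMatchStart swaps it for health, player info and a toggleable store.
; Click input drives hold-to-follow or short-press move; holding the pre-attack key shows attack range and routes attack clicks into that logic.
; QWER sends cursor locations to SkillComponent, and Tick shows a crosshair over minions.
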(event `self.ReceiveBeginPlay`
  ; 초기화
  (if (`self.IsLocalPlayerController`)
    (`parent.ReceiveBeginPlay`)
    (bind _returnvalue (`|CreateWidget` "/Game/LOL/UI/ChampSelect/WBP_ChampSelect.WBP_ChampSelect_C"))
    (set `self.ChampSelectWidget` _returnvalue)
    (`UserWidget.AddToViewport` (`self.ChampSelectWidget`) 0)
    (`WidgetBlueprintLibrary.SetInputMode_UIOnlyEx` self null)))

(event `Client_OnMatchStart`
  (`Widget.RemoveFromParent` (`self.ChampSelectWidget`))
  (`WidgetBlueprintLibrary.SetInputMode_GameAndUIEx` self null)
  ; 초기화
  (bind _returnvalue (`|CreateWidget` "/Game/LOL/UI/Characters/WBP_PlayerDetailHealth.WBP_PlayerDetailHealth_C" null (`/Game/LOL/Character/Champions/Ezreal/BP_Ezreal.BP_HealthPointsComponent` (`self.PlayerRef`))))
  (set `self.PlayerHealth` _returnvalue)
  (bind _returnvalue_2 (`|CreateWidget` "/Game/LOL/UI/Characters/WBP_PlayerInfo.WBP_PlayerInfo_C"))
  (set `self.PlayerInfoWidget` _returnvalue_2)
  (bind _returnvalue_3 (`|CreateWidget` "/Game/LOL/UI/Store/WBP_Store.WBP_Store_C"))
  (set `self.WBP Store` _returnvalue_3)
  (`KismetArrayLibrary.Array_Resize` (`/Game/LOL/Store/Blueprints/BP_InventoryComponent.Slots` (`/Game/LOL/Character/Champions/Ezreal/BP_Ezreal.BP_InventoryComponent` (`self.PlayerRef`))) (`self.InventorySize`))
  (`UserWidget.AddToViewport` (`self.PlayerHealth`) 0)
  (`UserWidget.AddToViewport` (`self.PlayerInfoWidget`) 0)
  (`UserWidget.AddToViewport` (`self.WBP Store`) 1)
  (`self.HideStore`))

(event `EnhancedInput|/Game/LOL/Input/Actions/IA_OpenShore`
  (params (ActionValue :type Boolean) (ElapsedSeconds :type "Float (double-precision)") (TriggeredSeconds :type "Float (double-precision)") (InputAction :type "InputAction Object Reference" :default "/Game/LOL/Input/Actions/IA_OpenShore.IA_OpenShore"))
  ; Store Button (P)
  (:`Triggered`
    (if (`Widget.IsVisible` (`self.WBP Store`))
      (`self.HideStore`)
      (else
        (`self.ShowStore`)))))

(event `HideStore`
  ; Hide Store
  (`Widget.SetVisibility` (`self.WBP Store`) "Hidden"))

(event `ShowStore`
  ; Show Store
  (`Widget.SetVisibility` (`self.WBP Store`) "Visible"))

(event `self.ReceiveTick`
  (params (DeltaSeconds :type "Float (single-precision)"))
  ; 마우스 커서의 대상이 미니언이면 커서 변경
  (`self.UpdateMouseCursor`))

(event `EnhancedInput|/Game/LOL/Input/Actions/IA_SetDestination_Click`
  (params (ActionValue :type Boolean) (ElapsedSeconds :type "Float (double-precision)") (TriggeredSeconds :type "Float (double-precision)") (InputAction :type "InputAction Object Reference" :default "/Game/LOL/Input/Actions/IA_SetDestination_Click.IA_SetDestination_Click"))
  (bind (_hit _location) (`self.GetLocationUnderCursor`))
  (bind (_hit_2 _location_2) (`self.GetLocationUnderCursor`))
  (bind _playerref (`self.PlayerRef`))
  ; TopDown Move
  (:`Triggered`
    (if _hit
      (bind _output_get (set `self.CachedDestination` _location))
      (`self.Follow` _output_get)))
  (:`Started`
    (`self.StopMovement` :!label _label)
    (if _hit_2
      (set `self.CachedDestination` _location_2)))
  (:`Canceled`
    (if (< (stale `EnhancedInput|/Game/LOL/Input/Actions/IA_AttackClick` ElapsedSeconds) (`self.PressedThreshold`)) :!label _label_2
      (`self.MoveTo` (`self.CachedDestination`))
      (if (`self.bIsNotAttackClick`)
        (set `/Game/LOL/Character/ActorComponents/AttackSystem/BP_AttackerComponent.TargetToAttack` null (`/Game/LOL/Character/Champions/Ezreal/BP_Ezreal.BP_AttackerComponent` _playerref))
        (`/Game/LOL/Character/Champions/Ezreal/BP_Ezreal.ResetAttackTimer` _playerref))))
  (:`Completed`
    (goto _label_2)))

(event `EnhancedInput|/Game/LOL/Input/Actions/IA_SkillQ`
  (params (ActionValue :type Boolean) (ElapsedSeconds :type "Float (double-precision)") (TriggeredSeconds :type "Float (double-precision)") (InputAction :type "InputAction Object Reference" :default "/Game/LOL/Input/Actions/IA_SkillQ.IA_SkillQ"))
  ; Ability Input QWER
  (:`Started`
    (bind _output_get (set `self.CachedDestination` (`.Location` (`self.GetLocationUnderCursor`))))
    (`SkillComponent.RequestUseSkill` (`/Game/LOL/Character/Champions/Ezreal/BP_Ezreal.SkillComponent` (`self.PlayerRef`)) "Q" _output_get)))

(event `EnhancedInput|/Game/LOL/Input/Actions/IA_AttackClick`
  (params (ActionValue :type Boolean) (ElapsedSeconds :type "Float (double-precision)") (TriggeredSeconds :type "Float (double-precision)") (InputAction :type "InputAction Object Reference" :default "/Game/LOL/Input/Actions/IA_AttackClick.IA_AttackClick"))
  ; Attack 키(좌클릭)
  (:`Started`
    (if (`self.bIsPreAttackKey`)
      (goto _label)))
  (:`Canceled`
    (if (`self.bIsPreAttackKey`) :!label _label_3
      (goto _label_2)))
  (:`Completed`
    (goto _label_3)))

(event `EnhancedInput|/Game/LOL/Input/Actions/IA_SkillW`
  (params (ActionValue :type Boolean) (ElapsedSeconds :type "Float (double-precision)") (TriggeredSeconds :type "Float (double-precision)") (InputAction :type "InputAction Object Reference" :default "/Game/LOL/Input/Actions/IA_SkillW.IA_SkillW"))
  ; Ability Input QWER
  (:`Started`
    (bind _output_get (set `self.CachedDestination` (`.Location` (`self.GetLocationUnderCursor`))))
    (`SkillComponent.RequestUseSkill` (`/Game/LOL/Character/Champions/Ezreal/BP_Ezreal.SkillComponent` (`self.PlayerRef`)) "W" _output_get)))

(event `EnhancedInput|/Game/LOL/Input/Actions/IA_SkillE`
  (params (ActionValue :type Boolean) (ElapsedSeconds :type "Float (double-precision)") (TriggeredSeconds :type "Float (double-precision)") (InputAction :type "InputAction Object Reference" :default "/Game/LOL/Input/Actions/IA_SkillE.IA_SkillE"))
  ; Ability Input QWER
  (:`Started`
    (bind _output_get (set `self.CachedDestination` (`.Location` (`self.GetLocationUnderCursor`))))
    (`SkillComponent.RequestUseSkill` (`/Game/LOL/Character/Champions/Ezreal/BP_Ezreal.SkillComponent` (`self.PlayerRef`)) "E" _output_get)))

(event `EnhancedInput|/Game/LOL/Input/Actions/IA_SkillR`
  (params (ActionValue :type Boolean) (ElapsedSeconds :type "Float (double-precision)") (TriggeredSeconds :type "Float (double-precision)") (InputAction :type "InputAction Object Reference" :default "/Game/LOL/Input/Actions/IA_SkillR.IA_SkillR"))
  ; Ability Input QWER
  (:`Started`
    (bind _output_get (set `self.CachedDestination` (`.Location` (`self.GetLocationUnderCursor`))))
    (`SkillComponent.RequestUseSkill` (`/Game/LOL/Character/Champions/Ezreal/BP_Ezreal.SkillComponent` (`self.PlayerRef`)) "R" _output_get)))

(event `EnhancedInput|/Game/LOL/Input/Actions/IA_PreAttackKey`
  (params (ActionValue :type Boolean) (ElapsedSeconds :type "Float (double-precision)") (TriggeredSeconds :type "Float (double-precision)") (InputAction :type "InputAction Object Reference" :default "/Game/LOL/Input/Actions/IA_PreAttackKey.IA_PreAttackKey"))
  (bind _returnvalue (/ (`/Game/LOL/Character/ActorComponents/AttackSystem/BP_AttackerComponent.AttackRange` (`/Game/LOL/Character/Champions/Ezreal/BP_Ezreal.BP_AttackerComponent` (`self.PlayerRef`))) 50.0))
  ; A키(사거리 표시 && PreAttackKey)
  (:`Triggered`
    (set `self.bIsPreAttackKey` true :!label _label_4)
    (`SceneComponent.SetWorldScale3D` (`/Game/LOL/Character/Champions/Ezreal/BP_Ezreal.SeeRangeMesh` (`self.PlayerRef`)) (`KismetMathLibrary.MakeVector` _returnvalue _returnvalue 1.0))
    (`SceneComponent.SetVisibility` (`/Game/LOL/Character/Champions/Ezreal/BP_Ezreal.SeeRangeMesh` (`self.PlayerRef`)) true false))
  (:`Started`
    (goto _label_4))
  (:`Canceled`
    (set `self.bIsPreAttackKey` false :!label _label_5)
    (`SceneComponent.SetVisibility` (`/Game/LOL/Character/Champions/Ezreal/BP_Ezreal.SeeRangeMesh` (`self.PlayerRef`)) false false))
  (:`Completed`
    (goto _label_5)))

(fn `UpdateMouseCursor`
  (bind (_bblockinghit _binitialoverlap _time _distance _location _impactpoint _normal _impactnormal _physmat _hitactor) (`GameplayStatics.BreakHitResult` (`self.GetHitResultUnderCursorByChannel` "TraceTypeQuery1")))
  (if _bblockinghit
    (cast `/Game/LOL/Character/Minion/Blueprints/BP_Minion` _hitactor
      (:`then`
        ; 공격 커서
        (set `self.CurrentMouseCursor` "Crosshairs"))
      (:`CastFailed`
        ; 일반 커서
        (set `self.CurrentMouseCursor` "Default")))))

(fn `UserConstructionScript`
  (`parent.UserConstructionScript`))