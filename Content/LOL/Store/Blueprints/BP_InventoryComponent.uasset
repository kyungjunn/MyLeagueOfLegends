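; Inventory component for the LOL store that keeps items as name and amount entries in a Slots array.
; Helpers find stackable slots using max stack counts from DT_ItemDataes, check ownership and place items into the first zero-amount slot.
; DeleteItem finds an item by name, then overwrites its slot, via DecreaseSlotStack for stackables.
; AddItem1's stack/duplicate rules and IncreaseSlotStack's body are disconnected from their entries, so neither runs.
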(fn `AddItem1`
  (params (ItemAmount :type Integer) (ItemName :type Name) (bisStackable :type Boolean) (bisDuplicatable :type Boolean))
  (returns (IsAddFailed :type Boolean))
  (locals (AmountLeft :type Integer)))

(fn `AddToNewSlot`
  (params (Itemname :type Name) (Amount :type Integer))
  (`KismetArrayLibrary.Array_Set` (`self.Slots`) (`.EmptySlotIndex` (`self.CheckSlotEmpty`))))

(fn `CheckHasItem`
  (params (ItemName :type Name))
  (returns (HasItem :type Boolean) (ArrayIndex :type Integer))
  (for (_array_element _array_index) _
    (if (== (`.Name_3_2B0D28C945F6FC054F88D5A102035B9D` (break `/Game/LOL/Store/Blueprints/Structs/ST_InventorySlot` _array_element)) (`local.ItemName`))
      (return true _array_index)))
  (return false -1))

(fn `CheckSlotAddOrNot`
  (params (ItemName :type Name) (AmountLeft :type Integer))
  (returns (bisAddFailed :type Boolean))
  ; 남은 슬롯이 있는가?
  (if (`self.CheckSlotEmpty`)
    ; 새로운 슬롯 아이템 추가
    (`self.AddToNewSlot` (`local.ItemName`) 1)
    (`/Engine/EditorBlueprintResources/StandardMacros.DecrementInt` (`local.AmountLeft`)
      (:`  `
        (return false)))
    (else
      (set `self.bIsAddFailed` true)
      (return true))))

(fn `CheckSlotEmpty`
  (returns (IsSlotAvailable :type Boolean) (EmptySlotIndex :type Integer))
  (for (_array_element _array_index) _
    ; 슬롯의 아이템 개수가 0?
    (if (== (`.Amount_6_BE3D393C48C08181F36C14B8BDD49E52` (break `/Game/LOL/Store/Blueprints/Structs/ST_InventorySlot` _array_element)) 0)
      (return true _array_index)))
  ; 인벤토리 전부 찾아봤는데 개수가 0인 슬롯이 없다면 -1
  (return false -1))

(fn `DecreaseSlotStack`
  (params (Index :type Integer) (Amount :type Integer))
  (bind _index (`local.Index`))
  (if (< 0 2)
    ; 슬롯을 비워서 보내기
    (`KismetArrayLibrary.Array_Set` (`self.Slots`) _index)
    (else
      (`KismetArrayLibrary.Array_Set` (`self.Slots`) _index))))

(fn `DeleteItem`
  (params (ItemName :type Name) (bisStackable :type Boolean))
  (bind (_hasitem _arrayindex) (`self.CheckHasItem` ItemName))
  ; 같은 이름의 아이템이 있는가?
  (if _hasitem
    ; 스택형 아이템인가?
    (if (`local.bisStackable`)
      (`self.DecreaseSlotStack` _arrayindex -1)
      (else
        ; 슬롯을 비워서 보내기
        (`KismetArrayLibrary.Array_Set` (`self.Slots`) _arrayindex)))))

(fn `FindSlot`
  (params (ItemName :type Name))
  (returns (`Array Index` :type Integer) (FoundSlot :type Boolean))
  (for (_array_element _array_index) _
    (bind (_name _amount) (break `/Game/LOL/Store/Blueprints/Structs/ST_InventorySlot` _array_element))
    ; 인벤토리 슬롯에 있는 아이템 name과 클릭한 아이템 name과 같다면?
    (if (== _name (`local.ItemName`))
      ; 아이템의 최대 StackSize가 인벤토리에 있는 아이템 개수보다 적다면?
      (if (< _amount (`self.GetStackSize` (`local.ItemName`)))
        (return _array_index true))))
  (return -1 false))

(fn `GetStackSize`
  (params (ItemName :type Name))
  (returns (StackSize :type Integer))
  (bind _returnvalue (`|GetDataTableRow` "/Game/LOL/Store/Blueprints/DataTables/DT_ItemDataes.DT_ItemDataes" ItemName)
    (:`then`
      (return (`.MaxStackCount` (break `ItemData` _returnvalue))))
    (:`RowNotFound`
      (return -1))))

(fn `IncreaseSlotStack`
  (params (Index :type Integer) (Amount :type Integer :default 1)))