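; Player controller Blueprint that creates the player's HUD widget and handles the store open/close input.
; On BeginPlay it creates WBP_HUD and stores it as PlayerHUD, without adding it to the viewport here.
; The IA_OpenShore input alternates ShowStore and CloseStore on the HUD through a FlipFlop, updating BisStoreOpen.
; An unconnected older toggle that creates and shows WBP_Store directly remains in the graph but never runs.
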(event `self.ReceiveBeginPlay`
  ; 기본 HUD 생성
  (`parent.ReceiveBeginPlay`)
  (bind _returnvalue (`|CreateWidget` "/Game/Store/Widgets/WBP_HUD.WBP_HUD_C"))
  (set `self.PlayerHUD` _returnvalue))

(event `EnhancedInput|/Game/TopDown/Input/Actions/IA_OpenShore`
  (params (ActionValue :type Boolean) (ElapsedSeconds :type "Float (double-precision)") (TriggeredSeconds :type "Float (double-precision)") (InputAction :type "InputAction Object Reference" :default "/Game/TopDown/Input/Actions/IA_OpenShore.IA_OpenShore"))
  (bind _playerhud (`self.PlayerHUD`))
  (:`Started`
    (`/Engine/EditorBlueprintResources/StandardMacros.FlipFlop`
      (:`A`
        (`/Game/Store/Widgets/WBP_HUD.ShowStore` _playerhud)
        (set `self.bisStoreOpen` true))
      (:`B`
        (`/Game/Store/Widgets/WBP_HUD.CloseStore` _playerhud)
        (set `self.bisStoreOpen` false)))))

(fn `UserConstructionScript`
  (`parent.UserConstructionScript`))