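; Inventory component that stores items as name and amount pairs in a fixed number of slots, sized on BeginPlay.
; AddItem places items one unit at a time, topping up a matching slot below its max stack count from DT_ItemData.
; Otherwise it claims the first slot with zero amount, and flags failure and stops when none is free.
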(event `self.ReceiveBeginPlay`
  (`KismetArrayLibrary.Array_Resize` (`self.Slots`) (`self.InventorySize`)))

(fn `AddItem`
  (params (ItemAmount :type Integer) (ItemName :type Name))
  (locals (AmountLeft :type Integer))
  (set `local.AmountLeft` ItemAmount)
  (while (and (> (`local.AmountLeft`) 0) (not (`self.bIsAddFailed`)))
    (bind (_arrayindex _foundslot) (`self.FindSlot` ItemName))
    ; 인벤토리에서 아이템을 찾았다면?
    (if _foundslot
      (`self.IncreaseSlotStack` _arrayindex)
      (`/Engine/EditorBlueprintResources/StandardMacros.DecrementInt` (`local.AmountLeft`))
      (else
        ; 아이템을 인벤토리에 못 찾은경우 인벤토리에 남은 슬롯이 있다면?
        (if (`self.CheckSlotEmpty`)
          ; 새로운 슬롯 아이템 추가
          (`self.AddToNewSlot` (`local.ItemName`) 1)
          (`/Engine/EditorBlueprintResources/StandardMacros.DecrementInt` (`local.AmountLeft`))
          (else
            (set `self.bIsAddFailed` true)))))))

(fn `AddToNewSlot`
  (params (Itemname :type Name) (Amount :type Integer))
  (`KismetArrayLibrary.Array_Set` (`self.Slots`) (`.EmptySlotIndex` (`self.CheckSlotEmpty`)) (make `/Game/Store/Blueprints/Structs/ST_InventorySlot` Itemname Amount)))

(fn `CheckSlotEmpty`
  (returns (IsSlotAvailable :type Boolean) (EmptySlotIndex :type Integer))
  (for (_array_element _array_index) (`self.Slots`)
    ; 슬롯의 아이템 개수가 0?
    (if (== (`.Amount_6_BE3D393C48C08181F36C14B8BDD49E52` (break `/Game/Store/Blueprints/Structs/ST_InventorySlot` _array_element)) 0)
      (return true _array_index)))
  ; 인벤토리 전부 찾아봤는데 개수가 0인 슬롯이 없다면 -1
  (return false -1))

(fn `FindSlot`
  (params (ItemName :type Name))
  (returns (ArrayIndex :type Integer) (FoundSlot :type Boolean))
  (for (_array_element _array_index) (`self.Slots`)
    (bind (_name _amount) (break `/Game/Store/Blueprints/Structs/ST_InventorySlot` _array_element))
    ; 인벤토리 슬롯에 있는 아이템 name과 클릭한 아이템 name과 같다면?
    (if (== _name (`local.ItemName`))
      ; 아이템의 최대 StackSize가 인벤토리에 있는 아이템 개수보다 적다면?
      (if (< _amount (`self.GetStackSize` (`local.ItemName`)))
        (return _array_index true))))
  (return -1 false))

(fn `GetStackSize`
  (params (ItemName :type Name))
  (returns (StackSize :type Integer))
  (bind _returnvalue (`|GetDataTableRow` "/Game/Store/Blueprints/DataTables/DT_ItemData.DT_ItemData" ItemName)
    (:`then`
      (return (`.MaxStackCount_22_C667C3904DE587FB19EDC5B8B19213AE` (break `/Game/Store/Blueprints/Structs/ST_ItemData` _returnvalue))))
    (:`RowNotFound`
      (return -1))))

(fn `IncreaseSlotStack`
  (params (Index :type Integer) (Amount :type Integer :default 1))
  (bind (_name _amount) (break `/Game/Store/Blueprints/Structs/ST_InventorySlot` (`|GetArrayItem` (`self.Slots`) Index)))
  (`KismetArrayLibrary.Array_Set` (`self.Slots`) Index (make `/Game/Store/Blueprints/Structs/ST_InventorySlot` _name (+ _amount Amount))))